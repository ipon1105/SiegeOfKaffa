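; BP_Rock is a siege rock actor that plays a random impact sound when its Cube component hits something hard.
; The Cube's hit event ignores weak impulses, then plays one of four sounds from an array at the component's location.
; An IsSounding flag, reset in the construction script and cleared after a short delay, throttles repeated sounds during continuous collisions.
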(event OnComponentHit(Cube)
  (params (HitComponent :type Primitive%20Component%20Object%20Reference) (OtherActor :type Actor%20Object%20Reference) (OtherComp :type Primitive%20Component%20Object%20Reference) (NormalImpulse :type Vector :default "0, 0, 0") (Hit :type Hit%20Result%20Structure%20%28by%20ref%29))
  ;[1 1 1] При слабом импульсе не проигрыаем звук
  (if (> (Math|Vector|VectorLength NormalImpulse) 1e+04)
    ;[1 1 1] Проигрываем рандомный звук
    (if (not (Variables|Default|GetisSounding))
      (Audio|PlaySoundatLocation (Utilities|Array|Get(acopy) (Variables|Default|GetSound) (Math|Random|RandomIntegerinRange 0 3)) (Transformation|GetWorldLocation HitComponent) "0, 0, 0" 1.0 1.0 0.0 0 0 0)
      (Variables|Default|SetisSounding true)
      (Utilities|FlowControl|Delay 0.6)
      (Variables|Default|SetisSounding false))))

(event EventBeginPlay)

(event Collision|EventActorBeginOverlap
  (params (OtherActor :type Actor%20Object%20Reference)))

(event EventTick
  (params (DeltaSeconds :type Float%20%28single-precision%29)))

(fn ConstructionScript
  (Variables|Default|SetisSounding false))