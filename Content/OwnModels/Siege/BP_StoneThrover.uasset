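; BP_StoneThrover is a siege stone thrower that loads and fires a single rock once play begins.
; BeginPlay plays matching body and hand load animations, then calls Shoot after a fixed delay.
; Shoot plays the firing animations, spawns BP_Rock at the ShootPose transform and launches its Cube with an impulse.
; The impulse adds the rock's forward vector to the Impulse variable rather than scaling it, so facing barely steers it.
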(event EventBeginPlay
  (CallFunction|Load)
  (Utilities|FlowControl|Delay 5.0)
  (CallFunction|Shoot))

(event EventTick
  (params (DeltaSeconds :type Float%20%28single-precision%29)))

(fn ConstructionScript)

(fn Shoot
  (bind _shootpose (Variables|Default|GetShootPose))
  (bind _returnvalue (Transformation|GetWorldTransform _shootpose))
  (bind (_location _rotation _scale) (Math|Transform|BreakTransform _returnvalue))
  (bind (_roll _pitch _yaw) (Math|Rotator|BreakRotator _rotation))
  (Components|Animation|PlayAnimation (Variables|Default|GetStoneThrover_Body) "/Game/OwnModels/Siege/Animation/StoneThrover_Body_Shoot.StoneThrover_Body_Shoot" false)
  (Components|Animation|PlayAnimation (Variables|Default|GetStoneThrover_Hand) "/Game/OwnModels/Siege/Animation/StoneThrover_Hand_Shoot.StoneThrover_Hand_Shoot" false)
  (bind _returnvalue_2 (Game|SpawnActorfromClass "/Game/OwnModels/Siege/BP_Rock.BP_Rock_C" (Math|Transform|MakeTransform _location (Math|Rotator|MakeRotator (+ _roll 0.0) (+ _pitch 0.0) (+ _yaw 0.0)) _scale) "AlwaysSpawn" 0 0))
  (Physics|AddImpulse (Variables|/Game/OwnModels/Siege/BP_Rock.BP_Rock_C|GetCube _returnvalue_2) (+ (Transformation|GetActorForwardVector _returnvalue_2) (Variables|Default|Getimpulse)) "rock" false))

(fn Load
  (Components|Animation|PlayAnimation (Variables|Default|GetStoneThrover_Body) "/Game/OwnModels/Siege/Animation/StoneThrover_Body_Load.StoneThrover_Body_Load" false)
  (Components|Animation|PlayAnimation (Variables|Default|GetStoneThrover_Hand) "/Game/OwnModels/Siege/Animation/StoneThrover_Hand_Load.StoneThrover_Hand_Load" false))