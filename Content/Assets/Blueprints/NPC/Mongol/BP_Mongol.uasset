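; BP_Mongol is a Mongol enemy NPC that dies when hit by a bolt.
; On BeginPlay it stores the first Gate actor, sets health and starts Krik, a self-rescheduling war cry at random intervals while alive.
; Move and Attack events only play looping mesh animations, with no movement or damage logic here.
; A bolt overlapping the capsule reduces health; on death the bolt is destroyed and the mesh ragdolls briefly before removal.
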(event OnComponentBeginOverlap(CapsuleComponent)
  (params (OverlappedComponent :type Primitive%20Component%20Object%20Reference) (OtherActor :type Actor%20Object%20Reference) (OtherComp :type Primitive%20Component%20Object%20Reference) (OtherBodyIndex :type Integer) (bFromSweep :type Boolean) (SweepResult :type Hit%20Result%20Structure%20%28by%20ref%29))
  ;[1 1 1] Смерть монгола
  (bind _asbolt (Utilities|Casting|CastTobolt OtherActor))
  (if true
    (bind _output_get (Variables|Default|SetHealth (- (Variables|Default|GetHealth) 30)))
    (if (<= _output_get 0)
      (Utilities|FlowControl|Sequence
        (:then_0
          (Actor|DestroyActor _asbolt))
        (:then_1
          (Physics|SetSimulatePhysics (Variables|Character|GetMesh) true)
          (Utilities|FlowControl|Delay 1.0)
          (Actor|DestroyActor self))))))

(event Custom|Attack
  (params (TraceEnd :type Vector))
  ;[1 1 1] При атаке играем анимацию атаки
  (Components|Animation|PlayAnimation (Variables|Character|GetMesh) "/Game/Assets/Animation/NPC/Mongol/Mongol_Anim_attack.Mongol_Anim_attack" true))

(event Custom|Move
  (params (WorldDirection :type Vector) (ScaleValue :type Float%20%28single-precision%29))
  ;[1 1 1] При движении играем анимацию бега
  (Components|Animation|PlayAnimation (Variables|Character|GetMesh) "/Game/Assets/Animation/NPC/Mongol/Mongol_Anim_run.Mongol_Anim_run" true))

(event Custom|Krik
  ;[1 1 1] Клич каждый 10-23 секунды
  (Utilities|FlowControl|Delay (Math|Random|RandomFloatinRange 2e+01 4e+01))
  (if (not (<= (Variables|Default|GetHealth) 0))
    (Audio|PlaySoundatLocation "/Game/Assets/Audio/NPC/Mongol/attack.attack" (Transformation|GetActorLocation self) "0, 0, 0" 1.0 1.0 0.0 0 0 0)
    (CallFunction|Krik)))

(event EventBeginPlay
  (Utilities|FlowControl|Sequence
    (:then_0
      ;[1 1 1] Устанавливаем ворота
      (bind _outactors (Actor|GetAllActorsOfClass "/Game/Assets/Blueprints/Props/Fortress/Gate.Gate_C"))
      (Variables|Default|SetGate (Utilities|Array|Get(acopy) _outactors)))
    (:then_1
      ;[1 1 1] Запоняем атрибуты
      (Variables|Default|SetHealth 1)
      (CallFunction|Krik))))

(fn ConstructionScript)